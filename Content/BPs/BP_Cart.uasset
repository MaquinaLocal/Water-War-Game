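; BP_Cart is an actor that shuttles a cart back and forth along its local Y axis.
; Each Tick offsets the actor by speed and direction, and rolls both wheels, scaled by delta time.
; A Delay fed from Tick acts as a repeating timer that turns the Cart component 180 degrees and negates the direction, with a DoOnce that resets immediately.
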(event EventTick
  (params (DeltaSeconds :type Float%20%28single-precision%29))
  (Variables|Default|SetDelta%20Seconds DeltaSeconds)
  (Utilities|FlowControl|Sequence
    (:then_0
      (Transformation|AddActorLocalOffset (Math|Vector|MakeVector 0.0 (* (Variables|Default|GetDelta%20Seconds) (Variables|Default|GetCartSpeed) (Variables|Default|GetDirection)) 0.0) false false))
    (:then_1
      (Transformation|AddLocalRotation (Variables|Default|GetWheelR) (Math|Rotator|MakeRotator (* (Variables|Default|GetDelta%20Seconds) (Variables|Default|GetWheelRotation)) 0.0 0.0) false false)
      (Transformation|AddLocalRotation (Variables|Default|GetWheelL) (Math|Rotator|MakeRotator (* (Variables|Default|GetDelta%20Seconds) (Variables|Default|GetWheelRotation)) 0.0 0.0) false false))
    (:then_2
      (Utilities|FlowControl|Delay (Variables|Default|GetChangeDirDelay))
      (Utilities|FlowControl|DoOnce false :!label _label
        (:Completed
          (Transformation|AddWorldRotation (Variables|Default|GetCart) "0,180.000000, 0" false false)
          (Variables|Default|SetDirection (* (Variables|Default|GetDirection) -1.0))
          (goto _label Reset))))))

(fn ConstructionScript)